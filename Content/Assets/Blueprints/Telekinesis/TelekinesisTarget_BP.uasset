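; Physics object that can be lifted, pulled toward a point and thrown by telekinesis.
; Lift disables gravity on its StaticMesh, and ReachTarget applies a velocity-change impulse toward the given location, clamped by distance and scaled down for heavier masses.
; Push restores gravity, sets linear damping and launches the mesh along the player camera's forward vector with a mass-independent impulse.
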(fn `Lift`
  (`PrimitiveComponent.SetEnableGravity` (`self.StaticMesh`) false))

(fn `Push`
  (bind _staticmesh (`self.StaticMesh`))
  (`PrimitiveComponent.SetEnableGravity` _staticmesh true)
  (`PrimitiveComponent.SetLinearDamping` _staticmesh 0.2)
  (`PrimitiveComponent.AddImpulse` _staticmesh (* (`SceneComponent.GetForwardVector` (`PlayerCameraManager.TransformComponent` (`GameplayStatics.GetPlayerCameraManager` 0))) 3000.0) "None" true))

(fn `ReachTarget`
  (params (Target :type "Vector Structure"))
  (`PrimitiveComponent.AddImpulse` (`self.StaticMesh`) (* (`KismetMathLibrary.ClampVectorSize` (- Target (`self.K2_GetActorLocation`)) 0.0 1000.0) (`KismetMathLibrary.MapRangeClamped` (`PrimitiveComponent.GetMass` (`self.StaticMesh`)) 50.0 700.0 5.0 1.0)) "None" true))

(fn `UserConstructionScript`)