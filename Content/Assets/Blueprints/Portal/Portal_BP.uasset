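; Portal actor whose view plane displays a render texture through a dynamic material, with events to set or clear the texture and adjust its scale offset.
; When a teleport is used on a non-target portal, FixView turns on until a zero-length delay ends.
; While it is on, Tick shifts the plane along local X by camera side and proximity to the portal's width segment, otherwise re-centring it.
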(event `self.ReceiveBeginPlay`
  (bind _returnvalue (`PrimitiveComponent.CreateDynamicMaterialInstance` (`self.PortalView`) 0 "/Game/Assets/Blueprints/Portal/PortalView_M.PortalView_M" "None"))
  (bind _output_get (set `self.ViewMaterial` _returnvalue)))

(event `self.SetRTT`
  (params (RenderTexture :type "Texture Object Reference"))
  (`/Engine/EditorBlueprintResources/StandardMacros.IsValid` RenderTexture
    (:`Is Valid`
      (`MaterialInstanceDynamic.SetTextureParameterValue` (`self.ViewMaterial`) "PortalTexture" RenderTexture))))

(event `self.ClearRTT`
  (`MaterialInstanceDynamic.SetTextureParameterValue` (`self.ViewMaterial`) "PortalTexture" null))

(event `self.OnTeleportUsed`
  (params (isTarget :type Boolean))
  (if (not isTarget)
    (set `self.FixView` true)
    (`KismetSystemLibrary.Delay` 0.0)
    (set `self.FixView` false)))

(event `self.ReceiveTick`
  (params (DeltaSeconds :type "Float (single-precision)"))
  (bind _portalview (`self.PortalView`))
  (bind _returnvalue (`PlayerCameraManager.GetCameraLocation` (`GameplayStatics.GetPlayerCameraManager` 0)))
  (if (`self.FixView`)
    (`SceneComponent.K2_SetRelativeLocation` _portalview (* (`KismetMathLibrary.SelectVector` (-15.0 0.0 150.0) (15.0 0.0 150.0) (not (`self.IsPointInFrontOfPortal` _returnvalue))) (`KismetMathLibrary.MakeVector` (- 1.0 (`KismetMathLibrary.FClamp` (`KismetMathLibrary.NormalizeToRange` (`self.Point Distance To Portal` _returnvalue) 50.0 150.0))) 1.0 1.0)) false false)
    (else
      (`SceneComponent.K2_SetRelativeLocation` _portalview (0.0 0.0 150.0) false false))))

(event `self.SetMaterialScale`
  (params (scale :type "Float (single-precision)"))
  (`MaterialInstanceDynamic.SetScalarParameterValue` (`self.ViewMaterial`) "ScaleOffset" scale))

(fn `IsCameraFacingSameDirectionAsPortal`
  (returns (Result :type Boolean))
  (return (> (`KismetMathLibrary.Dot_VectorVector` (`SceneComponent.GetForwardVector` (`self.PortalView`)) (- (`SceneComponent.K2_GetComponentLocation` (`self.PortalView`)) (`PlayerCameraManager.GetCameraLocation` (`GameplayStatics.GetPlayerCameraManager` 0)))) 0.0)))

(fn `Point Distance To Portal`
  (params (Point :type "Vector Structure"))
  (returns (Dist :type "Float (double-precision)"))
  (bind _portalview (`self.PortalView`))
  (bind (_min _max) (`StaticMeshComponent.GetLocalBounds` _portalview))
  (bind _returnvalue (`SceneComponent.K2_GetComponentLocation` _portalview))
  (bind _returnvalue_2 (`SceneComponent.GetRightVector` _portalview))
  (bind _returnvalue_3 (`SceneComponent.K2_GetComponentScale` _portalview))
  (return (`KismetMathLibrary.GetPointDistanceToSegment` Point (+ _returnvalue (* _returnvalue_2 (.y (* _min _returnvalue_3)))) (+ _returnvalue (* _returnvalue_2 (.y (* _max _returnvalue_3)))))))

(fn `UserConstructionScript`)