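; SlicableActor_BP is an actor whose sphere mesh material receives slice-plane data from a nearby portal.
; Each tick it scans all Portal_BP actors for the closest, using a squared-distance minimum that is never reset.
; It passes that PortalView's position, normal and bounds to the material as vector parameters.
; The normal is negated when the actor is in front of the portal, so it follows the actor's side.
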(event `self.ReceiveTick`
  (params (DeltaSeconds :type "Float (single-precision)"))
  (bind _sphere (`self.Sphere`))
  (bind _sphere_2 (`self.Sphere`))
  (bind _closestportal (`self.ClosestPortal`))
  (bind _portalview (`Portal.PortalView` _closestportal))
  (bind (_origin _boxextent) (`KismetSystemLibrary.GetComponentBounds` (`Portal.PortalView` (`self.ClosestPortal`))))
  (bind _returnvalue (`SceneComponent.GetForwardVector` _portalview))
  (`|ExecutionSequence`
    (:`then_0`
      (bind _outactors (`GameplayStatics.GetAllActorsOfClass` "/Game/Portal/Portal_BP.Portal_BP_C"))
      (for _array_element _outactors
        (bind _returnvalue_2 (`self.GetSquaredDistanceTo` self _array_element))
        (if (< _returnvalue_2 (`self.MinDistanseSq`))
          (set `self.MinDistanseSq` _returnvalue_2)
          (set `self.ClosestPortal` _array_element))))
    (:`then_1`
      (`MeshComponent.SetVectorParameterValueOnMaterials` _sphere_2 "Pos" (`SceneComponent.K2_GetComponentLocation` _portalview))
      (`MeshComponent.SetVectorParameterValueOnMaterials` _sphere_2 "Normal" (select `bool` (`Portal.IsPointInFrontOfPortal` _closestportal (`self.K2_GetActorLocation`)) :`false` _returnvalue :`true` (* _returnvalue -1.0)))
      (`MeshComponent.SetVectorParameterValueOnMaterials` _sphere "BoxPos" _origin)
      (`MeshComponent.SetVectorParameterValueOnMaterials` _sphere "BoxBounds" (* _boxextent 2.0)))))

(fn `UserConstructionScript`)